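; BP_MyGameHud puts up the in-level game UI and handles score updates.
; On BeginPlay it caches the BP_MyGi game instance, then creates a WBP_GameLevel widget and adds it to the viewport.
; Its Score event writes NewVar into the game instance's GameScore and passes that value to the widget's PointUpdate, so the score is stored in the game instance rather than the HUD.
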(event `self.ReceiveBeginPlay`
  (`|ExecutionSequence`
    (:`then_0`
      (bind _asbp_my_gi (cast `/Game/BP_MyGi` (`GameplayStatics.GetGameInstance`)))
      (set `self.As BP My Gi` _asbp_my_gi))
    (:`then_1`
      (bind _returnvalue (`|CreateWidget` "/Game/WBP_GameLevel.WBP_GameLevel_C"))
      (bind _output_get (set `self.Ref GameWidget` _returnvalue))
      (`UserWidget.AddToViewport` _output_get 0))))

(event `Score`
  (bind _output_get (set `/Game/BP_MyGi.GameScore` (`self.NewVar`) (`self.As BP My Gi`)))
  (`/Game/WBP_GameLevel.PointUpdate` (`self.Ref GameWidget`) _output_get))

(fn `UserConstructionScript`)